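; BP_CityIns_2 is a ground effect Blueprint that lays out city ground tiles as instances of one InstancedStaticMesh.
; Its construction script loop adds scaled-up instances at a fixed spacing along X.
; The grid-style divide and modulo index math uses a width of one, so the layout collapses to a single row.
; The event graph holds no active logic.
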(fn `UserConstructionScript`
  (for _index (range 3)
    (`InstancedStaticMeshComponent.AddInstance` (`self.InstancedStaticMesh`) (`KismetMathLibrary.MakeTransform` (`KismetMathLibrary.MakeVector` (`KismetMathLibrary.Conv_IntToDouble` (- (* (/ _index 1) 1000) 100)) (`KismetMathLibrary.Conv_IntToDouble` (- (* (mod _index 1) 1000) 100))) (struct) (10.0 10.0 1.0)))))