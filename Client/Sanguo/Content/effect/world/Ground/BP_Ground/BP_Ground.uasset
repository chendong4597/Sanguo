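; BP_Ground is a world ground effect Blueprint with replicated parameters for rotation, sine width and height, division count, a param flag and a city-to-ground value.
; BeginPlay and every OnRep handler call SetMaterialParam, a single refresh point for initial setup and replicated changes.
; SetMaterialParam currently only prints a placeholder debug string, so no material parameters are applied here.
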(event `self.ReceiveBeginPlay`
  (`self.Set Material Param`))

(fn `OnRep_CityToGround`
  (`self.Set Material Param`))

(fn `OnRep_DivideNum`
  (`self.Set Material Param`))

(fn `OnRep_IsParam`
  (`self.Set Material Param`))

(fn `OnRep_RotaX`
  (`self.Set Material Param`))

(fn `OnRep_RotaY`
  (`self.Set Material Param`))

(fn `OnRep_SinHeight`
  (`self.Set Material Param`))

(fn `OnRep_SinWidth`
  (`self.Set Material Param`))

(fn `Set Material Param`
  (`KismetSystemLibrary.PrintString` "222222222222222"))

(fn `UserConstructionScript`)