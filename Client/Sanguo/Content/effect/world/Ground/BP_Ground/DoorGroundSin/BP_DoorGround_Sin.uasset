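; BP_DoorGround_Sin is a ground effect Blueprint, a sine-based door-ground variant that configures its plane's material.
; It overrides SetMaterialParam, calling the parent and then, if IsParam is set, creating a dynamic instance of Ground_Sin_Door_M on the Plane.
; That instance receives the actor's sine shape, rotation, division and city-to-ground variables as scalar parameters.
; BeginPlay only calls the parent, and the construction script is empty.
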(event `self.ReceiveBeginPlay`
  (`parent.ReceiveBeginPlay`))

(fn `Set Material Param`
  (`parent.Set Material Param`)
  (if (`self.IsParam`)
    (bind _returnvalue (`PrimitiveComponent.CreateDynamicMaterialInstance` (`self.Plane`) 0 "/Game/effect/world/Ground/Meterials/Ground_Sin_Door_M.Ground_Sin_Door_M" "None"))
    (`MaterialInstanceDynamic.SetScalarParameterValue` _returnvalue "SinWidth" (`self.SinWidth`))
    (`MaterialInstanceDynamic.SetScalarParameterValue` _returnvalue "SinHeigh" (`self.SinHeight`))
    (`MaterialInstanceDynamic.SetScalarParameterValue` _returnvalue "RotaX" (`self.RotaX`))
    (`MaterialInstanceDynamic.SetScalarParameterValue` _returnvalue "RotaY" (`self.RotaY`))
    (`MaterialInstanceDynamic.SetScalarParameterValue` _returnvalue "DivideNum" (`self.DivideNum`))
    (`MaterialInstanceDynamic.SetScalarParameterValue` _returnvalue "CityToGround" (`self.CityToGround`))))

(fn `UserConstructionScript`)