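; BP_StaFlower is a flower status-effect visual, apparently for buffs, that continuously spins a Plane component.
; Tick accumulates delta time in MBeRot, and each time it passes a short threshold it adds a fixed yaw step to the plane's relative rotation and resets the timer.
; The spin is therefore stepped and advances at most one step per frame, with no other gameplay logic.
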(event `self.ReceiveTick`
  (params (DeltaSeconds :type "Float (single-precision)"))
  (bind (_relativerotation_roll _relativerotation_pitch _relativerotation_yaw) (`KismetMathLibrary.BreakRotator` (`SceneComponent.RelativeRotation` (`self.Plane`))))
  (bind _output_get (set `self.mBeRot` (+ DeltaSeconds (`self.mBeRot`))))
  (if (> _output_get 0.05)
    (`SceneComponent.K2_SetRelativeRotation` (`self.Plane`) (`KismetMathLibrary.MakeRotator` _relativerotation_roll _relativerotation_pitch (+ _relativerotation_yaw 15.0)) false false)
    (set `self.mBeRot` 0.0)))

(fn `UserConstructionScript`)