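; BP_AddSpeed is the visual effect actor for a speed buff, attached to a parent actor such as a player.
; Every tick it shows the PKySpeedbuff component only while the attach parent moves faster than a small velocity threshold.
; For parents implementing IPlayer, it also queries IsRiding and sets the effect's relative height, placing it lower when riding.
; The graph only drives the effect's visibility and position and does not change movement speed.
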(event `self.ReceiveTick`
  (params (DeltaSeconds :type "Float (single-precision)"))
  (bind _p_ky_speedbuff (`self.P_ky_speedbuff`))
  (bind _returnvalue (`self.GetAttachParentActor` self))
  (`SceneComponent.SetHiddenInGame` (`self.P_ky_speedbuff`) (not (> (`KismetMathLibrary.VSize` (`self.GetVelocity` _returnvalue)) 50.0)) false)
  (bind _asiplayer (cast `IPlayer` _returnvalue))
  (bind _returnvalue_2 (`IPlayer.IsRiding` _asiplayer))
  (if _returnvalue_2
    (`SceneComponent.K2_SetRelativeLocation` _p_ky_speedbuff (0.0 0.0 -150.0) false false)
    (else
      (`SceneComponent.K2_SetRelativeLocation` _p_ky_speedbuff (0.0 0.0 -70.0) false false))))

(fn `UserConstructionScript`)