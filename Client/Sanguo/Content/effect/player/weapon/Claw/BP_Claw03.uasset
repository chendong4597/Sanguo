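; Claw weapon effect actor that sets up two orange-tinted blade particle effects on spawn.
; BeginPlay runs ReviseRotate with different offsets, feeding RotateZ into per-blade rotation vector parameters alongside a color, then initializes BladeEff and BladeEff1 with differing Y rotations.
; It finally raises the actor 200 units on Z, while Tick and construction only call the parent.
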(event `self.ReceiveBeginPlay`
  (bind (_returnvalue_x _returnvalue_y _returnvalue_z) (`KismetMathLibrary.BreakVector` (`self.K2_GetActorLocation`)))
  (bind _rotatez (`self.RotateZ`))
  (bind _rotatez_2 (`self.RotateZ`))
  (`parent.ReceiveBeginPlay`)
  (`self.ReviseRotate` 0.3)
  (`self.AddVectorEffParams` "ColorInit" (254.0 50.0 0.0))
  (`self.AddVectorEffParams` "BlaInitRotation" (`KismetMathLibrary.MakeVector` 0.0 0.05 _rotatez_2))
  (`self.AddVectorEffParams` "BlaInitRotation1" (`KismetMathLibrary.MakeVector` 0.0 0.05 _rotatez_2))
  (`self.AddVectorEffParams` "ColorInit1" (254.0 50.0 0.0))
  (`self.AddVectorEffParams` "BlaInitRotation2" (`KismetMathLibrary.MakeVector` 0.0 0.05 _rotatez_2))
  (`self.AddVectorEffParams` "BlaInitRotation3" (`KismetMathLibrary.MakeVector` 0.0 0.05 _rotatez_2))
  (`self.AddVectorEffParams` "ColorInit2" (254.0 50.0 0.0))
  (`self.AddVectorEffParams` "BlaInitRotation4" (`KismetMathLibrary.MakeVector` 0.0 0.05 _rotatez_2))
  (`self.AddVectorEffParams` "BlaInitRotation5" (`KismetMathLibrary.MakeVector` 0.0 0.05 _rotatez_2))
  (`self.Initialize` (`self.BladeEff`))
  (`self.ReviseRotate` -0.1)
  (`self.AddVectorEffParams` "ColorInit" (254.0 50.0 0.0))
  (`self.AddVectorEffParams` "BlaInitRotation" (`KismetMathLibrary.MakeVector` 0.0 0.55 _rotatez))
  (`self.AddVectorEffParams` "BlaInitRotation1" (`KismetMathLibrary.MakeVector` 0.0 0.55 _rotatez))
  (`self.AddVectorEffParams` "ColorInit1" (254.0 50.0 0.0))
  (`self.AddVectorEffParams` "BlaInitRotation2" (`KismetMathLibrary.MakeVector` 0.0 0.55 _rotatez))
  (`self.AddVectorEffParams` "BlaInitRotation3" (`KismetMathLibrary.MakeVector` 0.0 0.55 _rotatez))
  (`self.AddVectorEffParams` "ColorInit2" (254.0 50.0 0.0))
  (`self.AddVectorEffParams` "BlaInitRotation4" (`KismetMathLibrary.MakeVector` 0.0 0.55 _rotatez))
  (`self.AddVectorEffParams` "BlaInitRotation5" (`KismetMathLibrary.MakeVector` 0.0 0.55 _rotatez))
  (`self.Initialize` (`self.BladeEff1`))
  (`self.K2_SetActorLocation` (`KismetMathLibrary.MakeVector` _returnvalue_x _returnvalue_y (+ _returnvalue_z 200.0))))

(event `self.ReceiveTick`
  (params (DeltaSeconds :type "Float (single-precision)"))
  (`parent.ReceiveTick` DeltaSeconds))

(fn `UserConstructionScript`
  (`parent.UserConstructionScript`))