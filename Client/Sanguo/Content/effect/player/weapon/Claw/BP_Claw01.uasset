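; Player claw weapon effect Blueprint that configures and starts a blade particle effect through functions it inherits.
; On BeginPlay it calls ReviseRotate, then registers vector parameters for the effect: the same orange initial color for several color slots and RotateZ-based initial rotations for several blade slots.
; It then passes BladeEff to Initialize.
; Tick and the construction script only defer to the parent.
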(event `self.ReceiveBeginPlay`
  (bind _rotatez (`self.RotateZ`))
  (`parent.ReceiveBeginPlay`)
  (`self.ReviseRotate` 0.2)
  (`self.AddVectorEffParams` "ColorInit" (254.0 50.0 0.0))
  (`self.AddVectorEffParams` "BlaInitRotation" (`KismetMathLibrary.MakeVector` 0.0 0.05 _rotatez))
  (`self.AddVectorEffParams` "BlaInitRotation1" (`KismetMathLibrary.MakeVector` 0.0 0.05 _rotatez))
  (`self.AddVectorEffParams` "ColorInit1" (254.0 50.0 0.0))
  (`self.AddVectorEffParams` "BlaInitRotation2" (`KismetMathLibrary.MakeVector` 0.0 0.05 _rotatez))
  (`self.AddVectorEffParams` "BlaInitRotation3" (`KismetMathLibrary.MakeVector` 0.0 0.05 _rotatez))
  (`self.AddVectorEffParams` "ColorInit2" (254.0 50.0 0.0))
  (`self.AddVectorEffParams` "BlaInitRotation4" (`KismetMathLibrary.MakeVector` 0.0 0.05 _rotatez))
  (`self.AddVectorEffParams` "BlaInitRotation5" (`KismetMathLibrary.MakeVector` 0.0 0.05 _rotatez))
  (`self.Initialize` (`self.BladeEff`)))

(event `self.ReceiveTick`
  (params (DeltaSeconds :type "Float (single-precision)"))
  (`parent.ReceiveTick` DeltaSeconds))

(fn `UserConstructionScript`
  (`parent.UserConstructionScript`))