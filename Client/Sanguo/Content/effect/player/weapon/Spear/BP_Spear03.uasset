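; BP_Spear03 is a player spear weapon effect built on a parent effect class and configured entirely in BeginPlay.
; It queues vector parameters for an initial color and ten initial rotations, calling ReviseRotate between pairs to vary the Z rotation.
; It then initializes the SpearEff01 effect with those parameters and clears the list.
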(event `self.ReceiveBeginPlay`
  (bind _rotatez (`self.RotateZ`))
  (bind _rotatez_2 (`self.RotateZ`))
  (bind _rotatez_3 (`self.RotateZ`))
  (bind _rotatez_4 (`self.RotateZ`))
  (bind _rotatez_5 (`self.RotateZ`))
  (`parent.ReceiveBeginPlay`)
  (`self.ReviseRotate` 0.0)
  (`self.AddVectorEffParams` "ColorInit" (50.0 20.0 0.5))
  (`self.AddVectorEffParams` "BlaInitRotation1" (`KismetMathLibrary.MakeVector` 0.0 0.0 _rotatez))
  (`self.AddVectorEffParams` "BlaInitRotation2" (`KismetMathLibrary.MakeVector` 0.0 0.0 _rotatez))
  (`self.ReviseRotate` -0.05)
  (`self.AddVectorEffParams` "BlaInitRotation3" (`KismetMathLibrary.MakeVector` 0.0 0.0 _rotatez_2))
  (`self.AddVectorEffParams` "BlaInitRotation4" (`KismetMathLibrary.MakeVector` 0.0 0.0 _rotatez_2))
  (`self.ReviseRotate` 0.1)
  (`self.AddVectorEffParams` "BlaInitRotation5" (`KismetMathLibrary.MakeVector` 0.0 0.0 _rotatez_3))
  (`self.AddVectorEffParams` "BlaInitRotation6" (`KismetMathLibrary.MakeVector` 0.0 0.0 _rotatez_3))
  (`self.ReviseRotate` -0.03)
  (`self.AddVectorEffParams` "BlaInitRotation7" (`KismetMathLibrary.MakeVector` 0.0 0.0 _rotatez_4))
  (`self.AddVectorEffParams` "BlaInitRotation8" (`KismetMathLibrary.MakeVector` 0.0 0.0 _rotatez_4))
  (`self.ReviseRotate` -0.05)
  (`self.AddVectorEffParams` "BlaInitRotation9" (`KismetMathLibrary.MakeVector` 0.0 0.0 _rotatez_5))
  (`self.AddVectorEffParams` "BlaInitRotation10" (`KismetMathLibrary.MakeVector` 0.0 0.0 _rotatez_5))
  (`self.Initialize` (`self.SpearEff01`))
  (`self.ClearVectorEffParams`))

(fn `UserConstructionScript`
  (`parent.UserConstructionScript`))