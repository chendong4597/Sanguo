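; BP_Knife02 is a player knife weapon effect Blueprint that configures and starts a blade effect.
; On BeginPlay it runs the parent logic, then registers named vector parameters for initial color (orange-red) and two blade rotations driven by RotateZ.
; It then calls Initialize with BladeEff.
; Tick and the construction script only forward to the parent, and the overlap event is disabled.
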(event `self.ReceiveBeginPlay`
  (bind _rotatez (`self.RotateZ`))
  (`parent.ReceiveBeginPlay`)
  (`self.AddVectorEffParams` "ColorInit" (254.0 50.0 0.0))
  (`self.AddVectorEffParams` "BlaInitRotation" (`KismetMathLibrary.MakeVector` 0.0 0.98 _rotatez))
  (`self.AddVectorEffParams` "BlaInitRotation1" (`KismetMathLibrary.MakeVector` 0.0 0.98 _rotatez))
  (`self.Initialize` (`self.BladeEff`)))

(event `self.ReceiveTick`
  (params (DeltaSeconds :type "Float (single-precision)"))
  (`parent.ReceiveTick` DeltaSeconds))

(fn `UserConstructionScript`
  (`parent.UserConstructionScript`))