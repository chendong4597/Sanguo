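; BP_TwinSword03 is a player twin-sword weapon effect that spawns two orange-tinted particle effects at begin play.
; It builds on parent helpers, calling ReviseRotate and queuing vector parameters for color and initial rotation before initializing each effect.
; Parameters are cleared between the two so the second effect gets its own rotation revision and an added Y rotation component.
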(event `self.ReceiveBeginPlay`
  (bind _rotatez (`self.RotateZ`))
  (bind _rotatez_2 (`self.RotateZ`))
  (`parent.ReceiveBeginPlay`)
  (`self.ReviseRotate` 0.3)
  (`self.AddVectorEffParams` "ColorInit" (254.0 50.0 0.0))
  (`self.AddVectorEffParams` "BlaInitRotation" (`KismetMathLibrary.MakeVector` 0.0 0.0 _rotatez_2))
  (`self.AddVectorEffParams` "BlaInitRotation1" (`KismetMathLibrary.MakeVector` 0.0 0.0 _rotatez_2))
  (`self.Initialize` (`self.ParEffect`))
  (`self.ClearVectorEffParams`)
  (`self.ReviseRotate` 0.05)
  (`self.AddVectorEffParams` "ColorInit" (254.0 50.0 0.0))
  (`self.AddVectorEffParams` "BlaInitRotation" (`KismetMathLibrary.MakeVector` 0.0 0.5 _rotatez))
  (`self.AddVectorEffParams` "BlaInitRotation1" (`KismetMathLibrary.MakeVector` 0.0 0.5 _rotatez))
  (`self.Initialize` (`self.ParEffect1`)))

(fn `UserConstructionScript`)