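; BP_WeaponEffect is an actor Blueprint for player weapon effects that configures a particle effect and tracks its rotation.
; Initialize stores the particle and pushes float and vector parameters from GetEffParams into it by name.
; BeginPlay maps actor yaw to a normalized RotateZ, which ReviseRotate offsets with a single wrap into 0–1.
; DelayDestroy only records a time and flag, with no destroy logic in this graph.
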(event `self.ReceiveBeginPlay`
  (`self.InitEffRotate`)
  (`parent.ReceiveBeginPlay`))

(fn `DelayDestroy`
  (params (DestroyTm :type "Float (double-precision)"))
  (set `self.DelayDestroyTm` DestroyTm)
  (set `self.bDelayDestroy` true))

(fn `InitEffRotate`
  (bind (_returnvalue_roll _returnvalue_pitch _returnvalue_yaw) (`KismetMathLibrary.BreakRotator` (`self.K2_GetActorRotation`)))
  (set `self.RotateZ` (/ (+ _returnvalue_yaw 180.0) 360.0)))

(fn `Initialize`
  (params (ParticleEff :type "FXSystemComponent Object Reference"))
  (locals (info :type "StuWeaponEffInfo Structure"))
  (bind _m_partical (`self.m_Partical`))
  (set `self.m_Partical` ParticleEff)
  (bind _returnvalue (`self.GetEffParams`))
  (for _array_element _returnvalue
    (bind _output_get (set `local.info` _array_element))
    (switch `WEAPONEFFTPY` (`.emTpy` (break `StuWeaponEffInfo` _output_get))
      (:`WEAPONEFFTPY_F`
        (bind _returnvalue_2 (`KismetStringLibrary.Conv_StringToName` (break `StuWeaponEffInfo` _output_get)))
        (`FXSystemComponent.SetFloatParameter` _m_partical _returnvalue_2 (`.fValue` (break `StuWeaponEffInfo` _output_get))))
      (:`WEAPONEFFTPY_V`
        (`FXSystemComponent.SetVectorParameter` _m_partical _returnvalue_2 (`.vecParams` (break `StuWeaponEffInfo` _output_get)))))))

(fn `ReviseRotate`
  (params (fRiValue :type "Float (double-precision)"))
  (bind _rotatez (`self.RotateZ`))
  (set `self.RotateZ` (- (`self.RotateZ`) fRiValue))
  (if (> _rotatez 1.0)
    (set `self.RotateZ` (- _rotatez 1.0))
    (elif (< _rotatez 0.0)
      (set `self.RotateZ` (+ _rotatez 1.0)))))

(fn `UserConstructionScript`)