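; Dragon head effect actor for a Ball skill that plays an animated attack as soon as it spawns.
; BeginPlay starts the attack montage on the skeletal mesh at double speed and runs a timeline alongside it.
; The timeline track drives the mesh's relative scale and roll, then the scale is set to a fixed size when it finishes.
; It contains no collision, damage or tick logic.
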(event `self.ReceiveBeginPlay`
  (bind _skeletalmesh (`self.SkeletalMesh`))
  (`|PlayMontage` (`self.SkeletalMesh`) "/Game/Weapon/entry_s/Ball/Ball_Dragon/ball_Atk_Montage.ball_Atk_Montage" 2.0
    (:`then`
      (bind (_direction _newtrack_0) (`Timeline|Timeline_0` :`NewTime` 1.5)
        (:`Update`
          (`SceneComponent.SetRelativeScale3D` _skeletalmesh (+ (* (600.0 600.0 600.0) _newtrack_0) (300.0 300.0 300.0)))
          (`SceneComponent.K2_SetRelativeRotation` _skeletalmesh (`KismetMathLibrary.MakeRotator` (+ (* _newtrack_0 50.0) -50.0) 0.0 -90.0) false false))
        (:`Finished`
          (`SceneComponent.SetRelativeScale3D` _skeletalmesh (600.0 600.0 600.0)))))))

(fn `UserConstructionScript`)