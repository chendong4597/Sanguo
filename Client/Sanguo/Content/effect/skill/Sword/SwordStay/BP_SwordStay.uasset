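; BP_SwordStay is a sword skill effect Blueprint that shows a continuously spinning mesh.
; On BeginPlay it runs the parent logic, then registers four timed events within the first second through AddTimeEvent, with no handling of them in this graph.
; Tick accumulates a frame-rate-independent angle and applies it as the StaticMesh's relative yaw, with a fixed roll laying the mesh on its side.
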(event `self.ReceiveBeginPlay`
  (`parent.ReceiveBeginPlay`)
  (`self.AddTimeEvent` 0.52)
  (`self.AddTimeEvent` 0.75)
  (`self.AddTimeEvent` 0.85)
  (`self.AddTimeEvent` 0.95))

(event `self.ReceiveTick`
  (params (DeltaSeconds :type "Float (single-precision)"))
  (bind _output_get (set `self.Rot` (+ (* 1000 DeltaSeconds) (`self.Rot`))))
  (`SceneComponent.K2_SetRelativeRotation` (`self.StaticMesh`) (`KismetMathLibrary.MakeRotator` 90.0 0.0 _output_get) false false))

(fn `UserConstructionScript`)