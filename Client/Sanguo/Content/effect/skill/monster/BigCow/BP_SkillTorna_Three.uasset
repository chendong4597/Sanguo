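; BP_SkillTorna_Three is a BigCow monster skill effect, apparently one of three tornadoes fired in a fan.
; On InitSkillEvent, InitRot offsets the start-to-target yaw by 30 degrees per skill index, centred on index 1.
; It projects a new target along that direction at the original 3D distance, keeping the target's Z, then turns the actor to face it.
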(event `self.InitSkillEvent`
  (`self.InitRot`))

(fn `InitRot`
  (bind (_m_targetpos_x _m_targetpos_y _m_targetpos_z) (`KismetMathLibrary.BreakVector` (`self.m_targetPos`)))
  (bind (_m_startpos_x _m_startpos_y) (`KismetMathLibrary.BreakVector` (`self.m_startPos`)))
  (bind _m_startpos (`self.m_startPos`))
  (bind _m_targetpos (`self.m_targetPos`))
  (bind (_returnvalue_roll _returnvalue_pitch _returnvalue_yaw) (`KismetMathLibrary.BreakRotator` (`KismetMathLibrary.FindLookAtRotation` _m_startpos _m_targetpos)))
  (bind _returnvalue (`KismetMathLibrary.Vector_Distance` _m_startpos _m_targetpos))
  (bind _returnvalue_2 (`self.GetSkillIdx`))
  (bind (_returnvalue_x _returnvalue_y) (`KismetMathLibrary.BreakVector` (`KismetMathLibrary.GetForwardVector` (`KismetMathLibrary.MakeRotator` _returnvalue_roll _returnvalue_pitch (+ (+ (* _returnvalue_2 30.0) -30.0) _returnvalue_yaw)))))
  (set `self.m_targetPos` (`KismetMathLibrary.MakeVector` (+ _m_startpos_x (* _returnvalue_x _returnvalue)) (+ _m_startpos_y (* _returnvalue_y _returnvalue)) _m_targetpos_z))
  (`self.K2_SetActorRotation` (`KismetMathLibrary.FindLookAtRotation` (`self.m_startPos`) (`self.m_targetPos`))))

(fn `UserConstructionScript`)