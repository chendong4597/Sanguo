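; Monster skill effect for the paladin statue, apparently a sword attack, that applies timed damage and moves a child actor vertically.
; On skill init it snaps to the X/Y of the actor returned by GetAttackRole.
; BeginPlay chains delays to call BPDamageDelay three times over five seconds.
; After the third call, a timeline drives the child actor's relative Z from a 500-unit downward offset.
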(event `self.ReceiveBeginPlay`
  (`KismetSystemLibrary.Delay` 0.1)
  (`self.BPDamageDelay`)
  (`KismetSystemLibrary.Delay` 1.5)
  (`self.BPDamageDelay`)
  (`KismetSystemLibrary.Delay` 3.4)
  (`self.BPDamageDelay`)
  (bind (_direction _newtrack_0) (`Timeline|Timeline_0` :!via `PlayFromStart`)
    (:`Update`
      (`SceneComponent.K2_SetRelativeLocation` (`self.ChildActor`) (`KismetMathLibrary.MakeVector` 0.0 0.0 (+ (* _newtrack_0 500.0) -500.0)) false false))))

(event `self.InitSkillEvent`
  (bind _returnvalue (`self.GetAttackRole`))
  (if (`KismetSystemLibrary.IsValid` _returnvalue)
    (bind (_returnvalue_x _returnvalue_y) (`KismetMathLibrary.BreakVector` (`self.K2_GetActorLocation` _returnvalue)))
    (`self.K2_SetActorLocation` (`KismetMathLibrary.MakeVector` _returnvalue_x _returnvalue_y))))

(fn `UserConstructionScript`)