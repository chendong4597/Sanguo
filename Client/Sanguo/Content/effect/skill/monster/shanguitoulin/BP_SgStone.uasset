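; BP_SgStone is a monster skill effect actor that places a stone on the target and deals delayed damage.
; On skill init it moves to the target role's location, then calls BPDamageDelay after a short delay if the target is valid.
; Separately, a timeline started on BeginPlay drives the Stone component's relative height, so the visual motion and damage timing are linked only by timing.
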(event `self.InitSkillEvent`
  (bind _returnvalue (`self.GetTargetRole`))
  (if (`KismetSystemLibrary.IsValid` _returnvalue)
    (`self.K2_SetActorLocation` (`self.K2_GetActorLocation` _returnvalue))
    (`KismetSystemLibrary.Delay` 0.8)
    (`self.BPDamageDelay`)))

(event `self.ReceiveBeginPlay`
  (bind (_direction _newtrack_0) (`Timeline|Timeline_0` :!via `PlayFromStart`)
    (:`Update`
      (`SceneComponent.K2_SetRelativeLocation` (`self.stone`) (`KismetMathLibrary.MakeVector` 0.0 0.0 (* _newtrack_0 1200.0)) false false))))

(fn `UserConstructionScript`)