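; BP_thunderMul is a monster skill effect for DraKingOri that shows a vertical beam, apparently thunder, at the target's position.
; On skill init it teleports itself once to the target role's location, if that role is valid.
; Every tick it re-reads its own location and sets the particle beam's source there, its endpoint a fixed height above, and both beam strengths.
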(event `self.ReceiveBeginPlay`
  (set `self.m_oriPos` (`self.K2_GetActorLocation`)))

(event `self.ReceiveTick`
  (params (DeltaSeconds :type "Float (single-precision)"))
  (bind _partical1 (`self.Partical1`))
  (bind (_m_oripos_x _m_oripos_y _m_oripos_z) (`KismetMathLibrary.BreakVector` (`self.m_oriPos`)))
  (set `self.m_oriPos` (`self.K2_GetActorLocation`))
  (`ParticleSystemComponent.SetBeamSourcePoint` (`self.Partical1`) 0 (`self.m_oriPos`) 0)
  (`ParticleSystemComponent.SetBeamTargetPoint` (`self.Partical1`) 0 (`KismetMathLibrary.MakeVector` _m_oripos_x _m_oripos_y (+ _m_oripos_z 500.0)) 0)
  (`ParticleSystemComponent.SetBeamSourceStrength` _partical1 0 0.3 0)
  (`ParticleSystemComponent.SetBeamTargetStrength` _partical1 0 0.3 0))

(event `self.InitSkillEvent`
  (bind _returnvalue (`self.GetTargetRole`))
  (if (`KismetSystemLibrary.IsValid` _returnvalue)
    (`self.K2_SetActorLocation` (`self.K2_GetActorLocation` _returnvalue))))

(fn `UserConstructionScript`)