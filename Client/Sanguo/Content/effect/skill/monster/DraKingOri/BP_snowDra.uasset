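; BP_snowDra is a DraKingOri monster skill effect that moves to its target role on skill init and spawns timed BP_rain actors around it.
; Each tick it slowly yaws and checks only the first VecParams entry, so the list must be time-ordered: XYZ is a doubled offset, W the spawn time.
; Spawned entries are removed, each rain receives the effect's Z as floor height, and the effect destroys itself after six seconds.
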(event `self.ReceiveBeginPlay`)

(event `self.InitSkillEvent`
  (bind _returnvalue (`self.GetTargetRole`))
  (if (`KismetSystemLibrary.IsValid` _returnvalue)
    (`self.K2_SetActorLocation` (`self.K2_GetActorLocation` _returnvalue))))

(event `self.ReceiveTick`
  (params (DeltaSeconds :type "Float (single-precision)"))
  (bind (_returnvalue_x _returnvalue_y _returnvalue_z) (`KismetMathLibrary.BreakVector` (`self.K2_GetActorLocation`)))
  (bind (_returnvalue_roll _returnvalue_pitch _returnvalue_yaw) (`KismetMathLibrary.BreakRotator` (`self.K2_GetActorRotation`)))
  ;[1 1 1] Comment
  (set `self.detTm` (+ (`self.detTm`) DeltaSeconds))
  (if (> (`self.detTm`) 6.0)
    (`self.K2_DestroyActor`)
    (else
      (`self.K2_SetActorRotation` (`KismetMathLibrary.MakeRotator` _returnvalue_roll _returnvalue_pitch (+ _returnvalue_yaw (* 2 DeltaSeconds))))
      (if (> (`KismetArrayLibrary.Array_Length` (`self.vecParams`)) 0)
        (for _index (range (+ (`KismetArrayLibrary.Array_Length` (`self.vecParams`)) 1))
          (bind (_x _y _z _w) (`KismetMathLibrary.BreakVector4` (`|GetArrayItem` (`self.vecParams`) _index)))
          (if (>= (`self.detTm`) _w)
            (bind _returnvalue (`|SpawnActorFromClass` "/Game/effect/skill/snow_rain/BP_rain.BP_rain_C" (`KismetMathLibrary.MakeTransform` (+ (* (`KismetMathLibrary.MakeVector` _x _y _z) 2.0) (`self.K2_GetActorLocation`))) "Undefined" "OverrideRootScale" self null))
            (bind _asbp_rain (cast `/Game/effect/skill/snow_rain/BP_rain` _returnvalue)
              (:`then`
                (`/Game/effect/skill/snow_rain/BP_rain.SetFloorZ` _asbp_rain _returnvalue_z))
              (:`CastFailed`
                _))
            (`KismetArrayLibrary.Array_Remove` (`self.vecParams`) _index)
            (break)
            (else
              (break))))))))

(fn `UserConstructionScript`)