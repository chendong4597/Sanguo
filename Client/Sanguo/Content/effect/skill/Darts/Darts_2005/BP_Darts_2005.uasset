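; BP_Darts_2005 is a dart skill effect that fans its target point out by skill index.
; On skill init, index 1 rotates MTargetPos 45 degrees around MStartPos and index 2 rotates it -45 degrees, leaving other indices unchanged.
; The rotation uses atan2 and sine/cosine in the XY plane, preserving horizontal distance and Z.
; BeginPlay runs the parent logic, then registers a half-second time event.
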(event `self.ReceiveBeginPlay`
  (`parent.ReceiveBeginPlay`)
  (`self.AddTimeEvent` 0.5))

(event `self.InitSkillEvent`
  (bind (_m_startpos_x _m_startpos_y) (`KismetMathLibrary.BreakVector` (`self.m_startPos`)))
  (bind (_m_targetpos_x _m_targetpos_y) (`KismetMathLibrary.BreakVector` (`self.m_targetPos`)))
  (bind (_m_startpos_x_2 _m_startpos_y_2) (`KismetMathLibrary.BreakVector` (`self.m_startPos`)))
  (bind (_m_targetpos_x_2 _m_targetpos_y_2 _m_targetpos_z) (`KismetMathLibrary.BreakVector` (`self.m_targetPos`)))
  (bind _returnvalue (`KismetMathLibrary.VSizeXY` (- (`self.m_targetPos`) (`self.m_startPos`))))
  (bind _returnvalue_2 (+ (`KismetMathLibrary.DegAtan2` (- _m_targetpos_y _m_startpos_y) (- _m_targetpos_x _m_startpos_x)) (`self.Degree`)))
  (bind _returnvalue_3 (+ _m_startpos_y_2 (* (`KismetMathLibrary.DegSin` _returnvalue_2) _returnvalue)))
  (bind _returnvalue_4 (+ _m_startpos_x_2 (* (`KismetMathLibrary.DegCos` _returnvalue_2) _returnvalue)))
  (bind _returnvalue_5 (`self.GetSkillIdx`))
  (switch `int` _returnvalue_5
    (:`1`
      (set `self.Degree` 45.0)
      (set `self.m_targetPos` (`KismetMathLibrary.MakeVector` _returnvalue_4 _returnvalue_3 _m_targetpos_z)))
    (:`2`
      (set `self.Degree` -45.0)
      (set `self.m_targetPos` (`KismetMathLibrary.MakeVector` _returnvalue_4 _returnvalue_3 _m_targetpos_z)))))

(fn `UserConstructionScript`)