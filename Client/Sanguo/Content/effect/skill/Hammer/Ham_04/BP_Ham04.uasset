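; Hammer skill effect actor that swings a hammer down and deals timed, widening area damage.
; On BeginPlay a timeline pitches the child actor through 90 degrees, then hides the HammerCyle component.
; Tick accumulates elapsed time and fires three one-shot BPDamageIndex hits as thresholds are crossed, calling the parent Tick only on the last.
; A delayed ground-impact particle swap is present but unconnected.
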(event `self.ReceiveBeginPlay`
  (bind (_direction _alph) (`Timeline|Timeline_0`)
    (:`Update`
      (`SceneComponent.K2_SetRelativeRotation` (`self.ChildActor`) (`KismetMathLibrary.MakeRotator` 0.0 (* -90 _alph)) false false))
    (:`Finished`
      (`SceneComponent.SetVisibility` (`self.HammerCyle`) false false))))

(event `self.ReceiveTick`
  (params (DeltaSeconds :type "Float (single-precision)"))
  (bind _fcurtm (`self.fCurTm`))
  (set `self.fPreTm` _fcurtm)
  (set `self.fCurTm` (+ DeltaSeconds _fcurtm))
  (if (and (>= (`self.fCurTm`) 0.7) (< (`self.fPreTm`) 0.7))
    (`self.BPDamageIndex` 1 600))
  (if (and (>= (`self.fCurTm`) 0.9) (< (`self.fPreTm`) 0.9))
    (`self.BPDamageIndex` 2 800))
  (if (and (>= (`self.fCurTm`) 1.2) (< (`self.fPreTm`) 1.2))
    (`self.BPDamageIndex` 2 1200)
    (`parent.ReceiveTick` 0.0)))

(fn `UserConstructionScript`)