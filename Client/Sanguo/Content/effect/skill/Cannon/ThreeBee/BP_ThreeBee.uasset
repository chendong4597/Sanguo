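; BP_ThreeBee is a Cannon skill effect actor that hosts three magic range effects as child actors.
; On BeginPlay it casts each child actor to SkillEffectMagicRange in sequence and gives it the same long maximum time through SetMaxTm.
; A failed cast stops the rest of the setup; overlap, tick and construction script hold no logic.
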(event `self.ReceiveActorBeginOverlap`
  (params (OtherActor :type "Actor Object Reference")))

(event `self.ReceiveBeginPlay`
  (bind _asskill_effect_magic_range (cast `SkillEffectMagicRange` (`ChildActorComponent.ChildActor` (`self.ChildActor`))))
  (`SkillEffectMagicRange.SetMaxTm` _asskill_effect_magic_range 1000.0)
  (bind _asskill_effect_magic_range_2 (cast `SkillEffectMagicRange` (`ChildActorComponent.ChildActor` (`self.ChildActor1`))))
  (`SkillEffectMagicRange.SetMaxTm` _asskill_effect_magic_range_2 1000.0)
  (bind _asskill_effect_magic_range_3 (cast `SkillEffectMagicRange` (`ChildActorComponent.ChildActor` (`self.ChildActor2`))))
  (`SkillEffectMagicRange.SetMaxTm` _asskill_effect_magic_range_3 1000.0))

(fn `UserConstructionScript`)