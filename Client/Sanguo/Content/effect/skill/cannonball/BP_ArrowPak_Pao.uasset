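; Cannonball skill actor, apparently one projectile of a radial volley, that sets its own heading when the skill initializes.
; InitSkillEvent turns the skill index into a yaw in 36-degree steps with a one-degree offset, then places MTargetPos 2000 units from MStartPos along it at the same height.
; The actor then rotates to face that target; no movement or hit logic is defined here.
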(event `self.ReceiveBeginPlay`)

(event `self.InitSkillEvent`
  (bind _returnvalue (`self.K2_GetActorLocation`))
  (bind (_m_startpos_x _m_startpos_y _m_startpos_z) (`KismetMathLibrary.BreakVector` (`self.m_startPos`)))
  (bind _returnvalue_2 (`KismetMathLibrary.Vector_Distance` _returnvalue (+ _returnvalue (* (`self.GetActorForwardVector`) 2000.0))))
  (bind _returnvalue_3 (`self.GetSkillIdx`))
  (bind (_returnvalue_x _returnvalue_y) (`KismetMathLibrary.BreakVector` (`KismetMathLibrary.GetForwardVector` (`KismetMathLibrary.MakeRotator` 0.0 0.0 (+ (* _returnvalue_3 36.0) 1.0)))))
  (bind _output_get (set `self.m_targetPos` (`KismetMathLibrary.MakeVector` (+ (* _returnvalue_x _returnvalue_2) _m_startpos_x) (+ (* _returnvalue_y _returnvalue_2) _m_startpos_y) _m_startpos_z)))
  (`self.K2_SetActorRotation` (`KismetMathLibrary.FindLookAtRotation` (`self.m_startPos`) _output_get)))

(fn `UserConstructionScript`)