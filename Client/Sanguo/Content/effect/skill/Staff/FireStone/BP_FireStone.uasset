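; BP_FireStone is the staff Fire Stone skill effect, set up as a projectile that starts high above its target.
; On skill init, it offsets the start point from the initial target position horizontally toward the attacking role and raises it vertically.
; It moves the actor there and sets target, height and a short duration.
; No movement logic appears here; BeginPlay, overlap and Tick are unused.
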(event `self.InitSkillEvent`
  (bind (_initpos_x _initpos_y _initpos_z) (`KismetMathLibrary.BreakVector` (`self.InitPos`)))
  (bind _returnvalue (+ _initpos_z 2000.0))
  (bind _returnvalue_2 (`self.GetInitTargetPos`))
  (set `self.InitPos` _returnvalue_2)
  (bind _returnvalue_3 (`self.GetAttackRole`))
  (`/Engine/EditorBlueprintResources/StandardMacros.IsValid` _returnvalue_3
    (:`Is Valid`
      (bind (_returnvalue_x _returnvalue_y) (`KismetMathLibrary.BreakVector` (* (`KismetMathLibrary.GetForwardVector` (`KismetMathLibrary.FindLookAtRotation` (`self.InitPos`) (`self.K2_GetActorLocation` _returnvalue_3))) 2000.0)))
      (set `self.m_startPos` (`KismetMathLibrary.MakeVector` (+ _initpos_x _returnvalue_x) (+ _initpos_y _returnvalue_y) _returnvalue))
      (set `self.m_fBomeHei` _returnvalue)
      (set `self.m_targetPos` (`self.InitPos`))
      (`self.K2_SetActorLocation` (`self.m_startPos`))
      (set `self.m_allTm` 0.4))))

(fn `UserConstructionScript`)