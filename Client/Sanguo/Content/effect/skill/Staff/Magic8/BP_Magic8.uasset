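; BP_Magic8 is a Staff skill effect that sets up a path radiating from its parent skill effect.
; On InitSkillEvent it takes the parent effect's location as the start position.
; The target lies at a fixed horizontal distance, with the parent's yaw offset by 45 degrees per skill index, so successive indices fan out around the parent.
; The graph only sets these positions; it contains no movement or hit logic.
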(event `self.ReceiveBeginPlay`)

(event `self.InitSkillEvent`
  (bind _returnvalue (`self.GetParentSkillEffect`))
  (`/Engine/EditorBlueprintResources/StandardMacros.IsValid` _returnvalue
    (:`Is Valid`
      (set `self.m_startPos` (`self.K2_GetActorLocation` _returnvalue))
      (bind _returnvalue_2 (`self.GetSkillIdx`))
      (bind (_returnvalue_x _returnvalue_y _returnvalue_z) (`KismetMathLibrary.BreakVector` (`self.K2_GetActorLocation` _returnvalue)))
      (bind (_returnvalue_roll _returnvalue_pitch _returnvalue_yaw) (`KismetMathLibrary.BreakRotator` (`self.K2_GetActorRotation` _returnvalue)))
      (bind _returnvalue_3 (+ _returnvalue_yaw (`KismetMathLibrary.Conv_IntToDouble` (* _returnvalue_2 45))))
      (set `self.m_targetPos` (`KismetMathLibrary.MakeVector` (+ _returnvalue_x (* 3500 (`KismetMathLibrary.DegCos` _returnvalue_3))) (+ _returnvalue_y (* 3500 (`KismetMathLibrary.DegSin` _returnvalue_3))) _returnvalue_z)))))

(fn `UserConstructionScript`)