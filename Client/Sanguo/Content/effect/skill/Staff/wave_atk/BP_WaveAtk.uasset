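; BP_WaveAtk is a staff skill effect for a wave attack that deals damage over expanding distances in its first second.
; Tick accumulates elapsed time and compares previous with current time to fire BPDamageDistanceRange once per threshold, with a larger range each step.
; The final, widest hit is nested under the preceding threshold's branch, so it fires only if one frame crosses both.
; The parent Tick likewise runs only on that preceding threshold's frame.
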(event `self.ReceiveTick`
  (params (DeltaSeconds :type "Float (single-precision)"))
  (bind _fcurtm (`self.fCurTm`))
  (set `self.fPreTm` _fcurtm)
  (set `self.fCurTm` (+ DeltaSeconds _fcurtm))
  (if (and (>= (`self.fCurTm`) 0.2) (< (`self.fPreTm`) 0.2))
    (`self.BPDamageDistanceRange` 300))
  (if (and (>= (`self.fCurTm`) 0.4) (< (`self.fPreTm`) 0.4))
    (`self.BPDamageDistanceRange` 450))
  (if (and (>= (`self.fCurTm`) 0.6) (< (`self.fPreTm`) 0.6))
    (`self.BPDamageDistanceRange` 650))
  (if (and (>= (`self.fCurTm`) 0.8) (< (`self.fPreTm`) 0.8))
    (`self.BPDamageDistanceRange` 800)
    (if (and (>= (`self.fCurTm`) 0.9) (< (`self.fPreTm`) 0.9))
      (`self.BPDamageDistanceRange` 1100))
    (`parent.ReceiveTick` DeltaSeconds)))

(fn `UserConstructionScript`)