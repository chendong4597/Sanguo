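; BP_FlyAtk is a staff skill effect that sets randomized start and target points for a flying attack.
; On skill init it reads the parent skill effect's transform, placing the start near the parent and the target far along its forward vector.
; Both points get random yaw-scaled horizontal offsets and share one random height, with the start raised higher.
; The graph only sets these positions and contains no movement or hit logic.
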(event `self.ReceiveBeginPlay`)

(event `self.InitSkillEvent`
  (bind _hei (`self.Hei`))
  (set `self.Hei` (`KismetMathLibrary.RandomInteger` 400))
  (bind _returnvalue (`self.GetParentSkillEffect`))
  (`/Engine/EditorBlueprintResources/StandardMacros.IsValid` _returnvalue
    (:`Is Valid`
      (bind (_returnvalue_roll _returnvalue_pitch _returnvalue_yaw) (`KismetMathLibrary.BreakRotator` (`self.K2_GetActorRotation` _returnvalue)))
      (bind _returnvalue_2 (* (`KismetMathLibrary.RandomInteger` 400) (`KismetMathLibrary.DegCos` _returnvalue_yaw)))
      (bind _returnvalue_3 (* (`KismetMathLibrary.RandomInteger` 400) (`KismetMathLibrary.DegSin` _returnvalue_yaw)))
      (set `self.m_targetPos` (+ (+ (* (`self.GetActorForwardVector` _returnvalue) 3500.0) (`self.K2_GetActorLocation` _returnvalue)) (`KismetMathLibrary.MakeVector` _returnvalue_2 _returnvalue_3 (`KismetMathLibrary.Conv_IntToDouble` _hei))))
      (set `self.m_startPos` (+ (`self.K2_GetActorLocation` _returnvalue) (`KismetMathLibrary.MakeVector` _returnvalue_2 _returnvalue_3 (`KismetMathLibrary.Conv_IntToDouble` (+ _hei 500))))))))

(fn `UserConstructionScript`)