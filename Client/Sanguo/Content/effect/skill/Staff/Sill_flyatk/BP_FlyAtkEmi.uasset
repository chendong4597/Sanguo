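; BP_FlyAtkEmi is a staff fly-attack skill effect actor that deals repeated ranged damage while it exists.
; After a short delay from BeginPlay it enables damage, and Tick accumulates delta time to call BPDamageDisRange at a fixed interval with a set distance and range.
; Tick also calls the parent Tick, passing zero rather than the real delta time.
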(event `self.ReceiveBeginPlay`
  (`KismetSystemLibrary.Delay` 0.5)
  (set `self.bStartDamge` true))

(event `self.ReceiveTick`
  (params (DeltaSeconds :type "Float (single-precision)"))
  (bind _fcurtm (`self.fCurTm`))
  (if (`self.bStartDamge`)
    (set `self.fCurTm` (+ DeltaSeconds (`self.fCurTm`)))
    (if (> _fcurtm 0.9)
      (set `self.fCurTm` (- _fcurtm 0.9))
      (`self.BPDamageDisRange` 2500.0 700)))
  (`parent.ReceiveTick` 0.0))

(fn `UserConstructionScript`)