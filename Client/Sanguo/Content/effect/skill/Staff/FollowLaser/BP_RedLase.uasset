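; BP_RedLase is a staff skill effect for a red follow laser that aims at its target role.
; On BeginPlay it casts its child actor to SkillEffectMagicRange and sets that effect's max time to a long fixed value.
; Each Tick it rotates the whole actor to face the target, if valid, using a look-at rotation between height-offset points on both actors.
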(event `self.ReceiveBeginPlay`
  (bind _asskill_effect_magic_range (cast `SkillEffectMagicRange` (`ChildActorComponent.ChildActor` (`self.ChildActor`))))
  (`SkillEffectMagicRange.SetMaxTm` _asskill_effect_magic_range 1000.0))

(event `self.ReceiveTick`
  (params (DeltaSeconds :type "Float (single-precision)"))
  (bind _returnvalue (`self.GetTargetRole`))
  (`/Engine/EditorBlueprintResources/StandardMacros.IsValid` _returnvalue
    (:`Is Valid`
      (`self.K2_SetActorRotation` (`KismetMathLibrary.FindLookAtRotation` (+ (`self.K2_GetActorLocation`) (0.0 0.0 80.0)) (+ (`self.K2_GetActorLocation` _returnvalue) (0.0 0.0 70.0)))))))

(fn `UserConstructionScript`)