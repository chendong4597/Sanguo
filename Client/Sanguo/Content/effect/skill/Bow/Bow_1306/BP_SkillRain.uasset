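; BP_SkillRain is a bow skill effect Blueprint, apparently one projectile of a rain-style attack, that randomizes its own trajectory.
; On InitSkillEvent it reads the initial target position and sets MStartPos high above it with random horizontal scatter.
; MTargetPos gets a separate, wider scatter and a fixed world height rather than the target's Z.
; The graph contains no movement, collision or damage logic.
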(event `self.ReceiveBeginPlay`)

(event `self.InitSkillEvent`
  (bind _returnvalue (`self.GetInitTargetPos`))
  (set `self.m_startPos` (`KismetMathLibrary.MakeVector` (+ (.x _returnvalue) (- (* (`KismetMathLibrary.RandomFloat`) 800.0) 400.0)) (+ (.y _returnvalue) (- (* (`KismetMathLibrary.RandomFloat`) 800.0) 400.0)) (+ (.z _returnvalue) 1200.0)))
  (set `self.m_targetPos` (`KismetMathLibrary.MakeVector` (+ (.x _returnvalue) (- (* (`KismetMathLibrary.RandomFloat`) 1200.0) 600.0)) (+ (.y _returnvalue) (- (* (`KismetMathLibrary.RandomFloat`) 1200.0) 600.0)) 720.0)))

(fn `UserConstructionScript`)