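; Rain emitter for a bow skill that deals damage in timed pulses from above the skill's target.
; On BeginPlay it moves itself to a fixed height over the initial target position, then runs the parent BeginPlay.
; Tick accumulates time and uses previous/current threshold crossings to call BPDamageInteral once at each of three evenly spaced moments.
; The parent Tick is called only after the final pulse, with zero delta time.
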(event `self.ReceiveBeginPlay`
  (bind _returnvalue (`self.GetInitTargetPos`))
  (`self.K2_SetActorLocation` (`KismetMathLibrary.MakeVector` (.x _returnvalue) (.y _returnvalue) (+ (.z _returnvalue) 500.0)))
  (`parent.ReceiveBeginPlay`))

(event `self.ReceiveTick`
  (params (DeltaSeconds :type "Float (single-precision)"))
  (bind _fcurtm (`self.fCurTm`))
  (set `self.fPreTm` _fcurtm)
  (set `self.fCurTm` (+ DeltaSeconds _fcurtm))
  (if (and (>= (`self.fCurTm`) 0.4) (< (`self.fPreTm`) 0.4))
    (`self.BPDamageInteral`))
  (if (and (>= (`self.fCurTm`) 0.8) (< (`self.fPreTm`) 0.8))
    (`self.BPDamageInteral`))
  (if (and (>= (`self.fCurTm`) 1.2) (< (`self.fPreTm`) 1.2))
    (`self.BPDamageInteral`)
    (`parent.ReceiveTick` 0.0)))

(fn `UserConstructionScript`)