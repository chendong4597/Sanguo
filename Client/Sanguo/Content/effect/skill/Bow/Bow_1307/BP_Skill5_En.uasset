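; BP_Skill5_En is a bow skill effect actor that aims itself as one part of a fan spread from its parent skill effect.
; On skill init it moves to the parent's location and projects a target 3000 units along the parent's forward vector.
; The skill index offsets that target's yaw in 15-degree steps from -30, keeping start height.
; The actor then rotates to face the target.
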(event `self.ReceiveBeginPlay`)

(event `self.InitSkillEvent`
  (bind (_m_startpos_x _m_startpos_y _m_startpos_z) (`KismetMathLibrary.BreakVector` (`self.m_startPos`)))
  (bind _m_startpos (`self.m_startPos`))
  (bind _returnvalue (`self.GetParentSkillEffect`))
  (if (`KismetSystemLibrary.IsValid` _returnvalue)
    (bind _returnvalue_2 (`self.K2_GetActorLocation` _returnvalue))
    (`self.K2_SetActorLocation` _returnvalue_2)
    (set `self.m_startPos` _returnvalue_2)
    (bind _returnvalue_3 (+ (* (`self.GetActorForwardVector` _returnvalue) 3000.0) (`self.K2_GetActorLocation`)))
    (set `self.m_targetPos` _returnvalue_3)
    (bind _returnvalue_4 (`self.GetSkillIdx`))
    (bind (_returnvalue_roll _returnvalue_pitch _returnvalue_yaw) (`KismetMathLibrary.BreakRotator` (`KismetMathLibrary.FindLookAtRotation` _m_startpos _returnvalue_3)))
    (bind (_returnvalue_x _returnvalue_y) (`KismetMathLibrary.BreakVector` (`KismetMathLibrary.GetForwardVector` (`KismetMathLibrary.MakeRotator` _returnvalue_roll _returnvalue_pitch (+ (+ (* _returnvalue_4 15.0) -30.0) _returnvalue_yaw)))))
    (bind _returnvalue_5 (`KismetMathLibrary.Vector_Distance` _m_startpos _returnvalue_3))
    (bind _output_get (set `self.m_targetPos` (`KismetMathLibrary.MakeVector` (+ (* _returnvalue_x _returnvalue_5) _m_startpos_x) (+ (* _returnvalue_y _returnvalue_5) _m_startpos_y) _m_startpos_z)))
    (`self.K2_SetActorRotation` (`KismetMathLibrary.FindLookAtRotation` (`self.m_startPos`) _output_get))))

(fn `UserConstructionScript`)