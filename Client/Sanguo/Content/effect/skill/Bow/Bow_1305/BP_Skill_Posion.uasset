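; BP_Skill_Posion is a bow skill effect actor, named for poison, that sets its own target direction by skill index.
; On InitSkillEvent it offsets the actor's yaw by 36 degrees per index, so ten indices would form a full ring.
; It projects MTargetPos along that direction at the original start-to-target distance, flattened to the start height, then rotates the actor to face it.
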(event `self.ReceiveBeginPlay`)

(event `self.InitSkillEvent`
  (bind (_returnvalue_roll _returnvalue_pitch _returnvalue_yaw) (`KismetMathLibrary.BreakRotator` (`self.K2_GetActorRotation`)))
  (bind (_m_startpos_x _m_startpos_y _m_startpos_z) (`KismetMathLibrary.BreakVector` (`self.m_startPos`)))
  (bind _returnvalue (`KismetMathLibrary.Vector_Distance` (`self.m_startPos`) (`self.m_targetPos`)))
  (bind _returnvalue_2 (`self.GetSkillIdx`))
  (bind (_returnvalue_x _returnvalue_y) (`KismetMathLibrary.BreakVector` (`KismetMathLibrary.GetForwardVector` (`KismetMathLibrary.MakeRotator` _returnvalue_roll _returnvalue_pitch (+ (* _returnvalue_2 36.0) _returnvalue_yaw)))))
  (bind _output_get (set `self.m_targetPos` (`KismetMathLibrary.MakeVector` (+ (* _returnvalue_x _returnvalue) _m_startpos_x) (+ (* _returnvalue_y _returnvalue) _m_startpos_y) _m_startpos_z)))
  (`self.K2_SetActorRotation` (`KismetMathLibrary.FindLookAtRotation` (`self.m_startPos`) _output_get)))

(fn `UserConstructionScript`)