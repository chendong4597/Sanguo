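; LongBolt_BP is a skill-effect projectile that flies until it overlaps a Role or its lifetime expires.
; After a brief startup delay it applies the speed from SetLaserInfo to ProjectileMovement, with a random spawn offset currently zeroed out.
; A box overlap with a Role outside the ignore array spawns a blue explosion and destroys it, without applying damage.
; SetLaserInfo never stores its IngoreRoles input.
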(event `self.ReceiveBeginPlay`
  (bind _returnvalue (`KismetMathLibrary.RandomFloatInRange` 0.0))
  (bind _projectilemovement (`self.ProjectileMovement`))
  (bind _mspeed (`self.mSpeed`))
  ;[1 1 1] Offsets projectile spawn location by random float within range
  (`KismetSystemLibrary.Delay` 0.02)
  (set `ProjectileMovementComponent.InitialSpeed` _mspeed _projectilemovement)
  (set `ProjectileMovementComponent.MaxSpeed` _mspeed _projectilemovement)
  (`self.K2_AddActorWorldOffset` (`KismetMathLibrary.MakeVector` _returnvalue _returnvalue))
  (`KismetSystemLibrary.Delay` (`self.m_Tm`))
  (`self.K2_DestroyActor` :!label _label))

(event `self.Box.OnComponentBeginOverlap`
  (params (OverlappedComponent :type "PrimitiveComponent Object Reference") (OtherActor :type "Actor Object Reference") (OtherComp :type "PrimitiveComponent Object Reference") (OtherBodyIndex :type Integer) (bFromSweep :type Boolean) (SweepResult :type "HitResult Structure (by ref)"))
  ;[1 1 1] Offsets projectile spawn location by random float within range
  (bind _asrole (cast `Role` OtherActor))
  (if (== (`KismetArrayLibrary.Array_Find` (`self.IngoreArrayRole`) _asrole) -1)
    (bind _returnvalue (`Role.GetHitWorldTransform` _asrole))
    (`GameplayStatics.SpawnEmitterAtLocation` "/Game/effect/skill/BeamsAndLazers/Particles/P_Explosion_Blue.P_Explosion_Blue" (.location _returnvalue) (.rotation _returnvalue) (.scale _returnvalue))
    (goto _label)))

(fn `SetLaserInfo`
  (params (speed :type "Float (double-precision)") (tm :type "Float (double-precision)") (ingoreRoles :type "Array of Actor Object Reference"))
  (set `self.mSpeed` speed)
  (set `self.m_Tm` tm))

(fn `UserConstructionScript`)