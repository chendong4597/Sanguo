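; Red Triple Threat beam skill effect actor that hosts a StreamingBeam_BP_Red beam as a child actor.
; Shortly after BeginPlay it casts the StreamingBeamBP2 child and registers the targets from GetIngoreTargets, plus every AFort actor, as actors that beam ignores.
; Tick calls a world rotation with a zero delta, so that call produces no spin.
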(event `self.ReceiveTick`
  (params (DeltaSeconds :type "Float (single-precision)"))
  ;[1 1 1] Rotates Actor by tick
  (set `self.DeltaTime` DeltaSeconds)
  (`self.K2_AddActorWorldRotation` (struct)))

(event `self.ReceiveBeginPlay`
  ;[1 1 1] Comment
  (`KismetSystemLibrary.Delay` 0.01)
  (bind _returnvalue (`self.GetIngoreTargets`))
  (bind _asstreaming_beam_bp_red (cast `/Game/effect/skill/BeamsAndLazers/Blueprints/TripleThrea/StreamingBeam_BP_Red` (`ChildActorComponent.ChildActor` (`self.StreamingBeam_BP2`))))
  (`/Game/effect/skill/BeamsAndLazers/Blueprints/TripleThrea/StreamingBeam_BP_Red.AddIngoreActors` _asstreaming_beam_bp_red _returnvalue)
  (bind _outactors (`GameplayStatics.GetAllActorsOfClass` "/Script/ThirdReich.AFort"))
  (`/Game/effect/skill/BeamsAndLazers/Blueprints/TripleThrea/StreamingBeam_BP_Red.AddIngoreActors` _asstreaming_beam_bp_red _outactors))

(fn `UserConstructionScript`)