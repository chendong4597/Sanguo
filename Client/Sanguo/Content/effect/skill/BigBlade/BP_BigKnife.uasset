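; Big knife skill effect actor that animates a blade mesh in a fast downward swing.
; InitSkillEvent resets the swing angle and Alpha, and creates a dynamic instance of the knife material.
; Tick lowers the mesh pitch at a constant, frame-time-scaled rate until it clamps just below horizontal.
; Alpha keeps rising unclamped throughout, even after the swing stops, and feeds the material's "Alp" parameter.
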(event `self.ReceiveBeginPlay`)

(event `self.InitSkillEvent`
  (`SceneComponent.K2_SetRelativeRotation` (`self.StaticMesh`) (struct :`Pitch` 150.0) false false)
  (set `self.curRate` 90.0)
  (`PrimitiveComponent.CreateDynamicMaterialInstance` (`self.StaticMesh`) 0 "/Game/effect/skill/BigBlade/BigKnife_M.BigKnife_M" "0")
  (set `self.Alpha` 0.0))

(event `self.ReceiveTick`
  (params (DeltaSeconds :type "Float (single-precision)"))
  (bind _staticmesh (`self.StaticMesh`))
  (bind _currate (`self.curRate`))
  (bind _alpha (`self.Alpha`))
  (bind _returnvalue (- (`self.curRate`) (* 720 DeltaSeconds)))
  (bind _returnvalue_2 (+ (* DeltaSeconds 0.3) (`self.Alpha`)))
  (bind _output (`|GetArrayItem` (`MeshComponent.GetMaterials` _staticmesh)))
  (if (< _returnvalue -5.0)
    (set `self.curRate` -5.0)
    (`SceneComponent.K2_SetRelativeRotation` _staticmesh (`KismetMathLibrary.MakeRotator` 0.0 _currate) false false)
    (set `self.Alpha` _returnvalue_2)
    (bind _asmaterial_instance_dynamic (cast `MaterialInstanceDynamic` _output))
    (`MaterialInstanceDynamic.SetScalarParameterValue` _asmaterial_instance_dynamic "Alp" _alpha)
    (else
      (set `self.curRate` _returnvalue)
      (`SceneComponent.K2_SetRelativeRotation` _staticmesh (`KismetMathLibrary.MakeRotator` 0.0 _currate) false false)
      (set `self.Alpha` _returnvalue_2)
      (bind _asmaterial_instance_dynamic_2 (cast `MaterialInstanceDynamic` _output))
      (`MaterialInstanceDynamic.SetScalarParameterValue` _asmaterial_instance_dynamic_2 "Alp" _alpha))))

(fn `UserConstructionScript`)