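; Gun skill effect actor that plays a skill montage and deals damage over an advancing distance.
; On skill init it offsets its yaw by skill index, fanning instances out in fixed angular steps, then plays a sped-up montage, hiding the mesh and destroying the skill on completion.
; Tick grows a distance at constant speed, feeding it to BPDamageCircle and calling parent Tick only until it passes a maximum range.
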(event `self.InitSkillEvent`
  (bind (_returnvalue_roll _returnvalue_pitch _returnvalue_yaw) (`KismetMathLibrary.BreakRotator` (`self.K2_GetActorRotation`)))
  (bind _skeletalmesh (`self.SkeletalMesh`))
  (bind _returnvalue (`self.GetSkillIdx`))
  (`self.K2_SetActorRotation` (`KismetMathLibrary.MakeRotator` _returnvalue_roll _returnvalue_pitch (+ _returnvalue_yaw (`KismetMathLibrary.Conv_IntToDouble` (+ (* _returnvalue 30) -60)))))
  (`|PlayMontage` _skeletalmesh "/Game/effect/skill/Ball/Ball_Dragon/skill_Anim_Montage.skill_Anim_Montage" 3.5
    (:`OnCompleted`
      (`SceneComponent.SetHiddenInGame` _skeletalmesh true false)
      (`self.SkillDestroy`))))

(event `self.ReceiveTick`
  (params (DeltaSeconds :type "Float (single-precision)"))
  (bind _output_get (set `self.fDis` (+ (* DeltaSeconds 1800.0) (`self.fDis`))))
  (if (not (> _output_get 3000.0))
    (`self.BPDamageCircle` (`KismetMathLibrary.FTrunc` _output_get))
    (`parent.ReceiveTick` DeltaSeconds)))

(fn `UserConstructionScript`)