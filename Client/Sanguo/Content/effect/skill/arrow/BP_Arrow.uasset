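; Arrow skill projectile that runs on timeline logic from its parent skill class, with randomized target and arc.
; On skill init it hides the mesh, jitters the height parameter and horizontal target position, then waits in proportion to its skill index to stagger a volley.
; It then shows the mesh, enables the timeline and calls the parent BeginPlay.
; When the timeline ends, it spawns a blue beam impact effect at its location.
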(event `self.ReceiveBeginPlay`)

(event `self.InitSkillEvent`
  (bind (_m_targetpos_x _m_targetpos_y _m_targetpos_z) (`KismetMathLibrary.BreakVector` (`self.m_targetPos`)))
  (`SceneComponent.SetVisibility` (`self.StaticMesh`) false false)
  (set `self.m_bStartTmline` false)
  (set `self.m_fBomeHei` (+ (`self.m_fBomeHei`) (- (* (`KismetMathLibrary.RandomFloat`) 50.0) 25.0)))
  (set `self.m_targetPos` (`KismetMathLibrary.MakeVector` (+ _m_targetpos_x (- (* (`KismetMathLibrary.RandomFloat`) 500.0) 250.0)) (+ _m_targetpos_y (- (* (`KismetMathLibrary.RandomFloat`) 500.0) 250.0)) _m_targetpos_z))
  (bind _returnvalue (`self.GetSkillIdx`))
  (`KismetSystemLibrary.Delay` (* _returnvalue 0.05))
  (`SceneComponent.SetVisibility` (`self.StaticMesh`) true false)
  (set `self.m_bStartTmline` true)
  (`parent.ReceiveBeginPlay`))

(event `self.TimeLineEnd`
  (bind (_returnvalue_x _returnvalue_y _returnvalue_z) (`KismetMathLibrary.BreakVector` (`self.K2_GetActorLocation`)))
  (`GameplayStatics.SpawnEmitterAtLocation` "/Game/effect/skill/BeamsAndLazers/Particles/P_BlueBeamImpact.P_BlueBeamImpact" (`KismetMathLibrary.MakeVector` _returnvalue_x _returnvalue_y _returnvalue_z)))

(fn `UserConstructionScript`
  (`parent.UserConstructionScript`))