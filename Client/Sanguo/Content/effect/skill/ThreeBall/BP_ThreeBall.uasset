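; Skill effect actor that circles three BP_OneBall child actors around itself as damaging orbs.
; InitSkillEvent passes the attack role to each ball.
; Tick advances each ball's orbit by deriving its angle from its current relative location, keeping radius and height fixed.
; It also forwards the skill's attacker, range and ID to every ball's EvtDamage each frame, and calls EvtClear on them about once per second.
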(event `self.ReceiveBeginPlay`)

(event `self.InitSkillEvent`
  (bind _returnvalue (`self.GetAttackRole`))
  (bind _asbp_one_ball (cast `/Game/effect/skill/ThreeBall/BP_OneBall` (`ChildActorComponent.ChildActor` (`self.ChildActor`)))
    (:`then`
      (`self.SetBPAttackRole` _asbp_one_ball _returnvalue))
    (:`CastFailed`
      _))
  (bind _asbp_one_ball_2 (cast `/Game/effect/skill/ThreeBall/BP_OneBall` (`ChildActorComponent.ChildActor` (`self.ChildActor1`)))
    (:`then`
      (`self.SetBPAttackRole` _asbp_one_ball_2 _returnvalue))
    (:`CastFailed`
      _))
  (bind _asbp_one_ball_3 (cast `/Game/effect/skill/ThreeBall/BP_OneBall` (`ChildActorComponent.ChildActor` (`self.ChildActor2`))))
  (`self.SetBPAttackRole` _asbp_one_ball_3 _returnvalue))

(event `self.ReceiveTick`
  (params (DeltaSeconds :type "Float (single-precision)"))
  (bind _returnvalue (* 100 DeltaSeconds))
  (bind _childactor (`self.ChildActor`))
  (bind _curtm (`self.curTm`))
  (bind _childactor1 (`self.ChildActor1`))
  (bind _childactor2 (`self.ChildActor2`))
  (bind _returnvalue_2 (`SceneComponent.GetRelativeTransform` _childactor))
  (bind _returnvalue_3 (`SceneComponent.GetRelativeTransform` _childactor2))
  (bind _returnvalue_4 (`SceneComponent.GetRelativeTransform` _childactor1))
  (bind _returnvalue_5 (+ (`KismetMathLibrary.DegAtan2` (.x (.location _returnvalue_3)) (.y (.location _returnvalue_3))) _returnvalue))
  (bind _returnvalue_6 (+ (`KismetMathLibrary.DegAtan2` (.x (.location _returnvalue_2)) (.y (.location _returnvalue_2))) _returnvalue))
  (bind _returnvalue_7 (+ (`KismetMathLibrary.DegAtan2` (.x (.location _returnvalue_4)) (.y (.location _returnvalue_4))) _returnvalue))
  (`SceneComponent.K2_SetRelativeLocation` _childactor (`KismetMathLibrary.MakeVector` (* (`KismetMathLibrary.DegSin` _returnvalue_6) 700.0) (* (`KismetMathLibrary.DegCos` _returnvalue_6) 700.0) 150.0) false false)
  (`SceneComponent.K2_SetRelativeLocation` _childactor1 (`KismetMathLibrary.MakeVector` (* (`KismetMathLibrary.DegSin` _returnvalue_7) 700.0) (* (`KismetMathLibrary.DegCos` _returnvalue_7) 700.0) 150.0) false false)
  (`SceneComponent.K2_SetRelativeLocation` _childactor2 (`KismetMathLibrary.MakeVector` (* (`KismetMathLibrary.DegSin` _returnvalue_5) 700.0) (* (`KismetMathLibrary.DegCos` _returnvalue_5) 700.0) 150.0) false false)
  (`parent.ReceiveTick` DeltaSeconds)
  (bind _returnvalue_8 (`self.GetDamageSkillId`))
  (bind _returnvalue_9 (`self.GetDamageRange`))
  (bind _returnvalue_10 (`self.GetDamageAttacker`))
  (bind _asbp_one_ball (cast `/Game/effect/skill/ThreeBall/BP_OneBall` (`ChildActorComponent.ChildActor` (`self.ChildActor`)))
    (:`then`
      (`/Game/effect/skill/ThreeBall/BP_OneBall.EvtDamage` _asbp_one_ball _returnvalue_10 _returnvalue_9 _returnvalue_8))
    (:`CastFailed`
      _))
  (bind _asbp_one_ball_2 (cast `/Game/effect/skill/ThreeBall/BP_OneBall` (`ChildActorComponent.ChildActor` (`self.ChildActor1`)))
    (:`then`
      (`/Game/effect/skill/ThreeBall/BP_OneBall.EvtDamage` _asbp_one_ball_2 _returnvalue_10 _returnvalue_9 _returnvalue_8))
    (:`CastFailed`
      _))
  (bind _asbp_one_ball_3 (cast `/Game/effect/skill/ThreeBall/BP_OneBall` (`ChildActorComponent.ChildActor` (`self.ChildActor2`)))
    (:`then`
      (`/Game/effect/skill/ThreeBall/BP_OneBall.EvtDamage` _asbp_one_ball_3 _returnvalue_10 _returnvalue_9 _returnvalue_8))
    (:`CastFailed`
      _))
  (set `self.curTm` (+ DeltaSeconds (`self.curTm`)))
  (if (> _curtm 1.0)
    (set `self.curTm` (- _curtm 1.0))
    (bind _asbp_one_ball_4 (cast `/Game/effect/skill/ThreeBall/BP_OneBall` (`ChildActorComponent.ChildActor` (`self.ChildActor`)))
      (:`then`
        (`/Game/effect/skill/ThreeBall/BP_OneBall.EvtClear` _asbp_one_ball_4))
      (:`CastFailed`
        _))
    (bind _asbp_one_ball_5 (cast `/Game/effect/skill/ThreeBall/BP_OneBall` (`ChildActorComponent.ChildActor` (`self.ChildActor1`)))
      (:`then`
        (`/Game/effect/skill/ThreeBall/BP_OneBall.EvtClear` _asbp_one_ball_5))
      (:`CastFailed`
        _))
    (bind _asbp_one_ball_6 (cast `/Game/effect/skill/ThreeBall/BP_OneBall` (`ChildActorComponent.ChildActor` (`self.ChildActor2`))))
    (`/Game/effect/skill/ThreeBall/BP_OneBall.EvtClear` _asbp_one_ball_6)))

(fn `UserConstructionScript`)