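; Horse Blueprint under the weapon models that applies its coat textures to the skeletal mesh at runtime.
; On BeginPlay it creates dynamic instances of the shared Com_Weapon_M material on the first two material slots and sets their "Defuse" parameter to the Horse and Horse_prom textures.
; Tick, overlap and construction script add no logic beyond the parent class.
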(event `self.ReceiveBeginPlay`
  (bind _skeletalmesh (`self.SkeletalMesh`))
  (`parent.ReceiveBeginPlay`)
  (bind _returnvalue (`PrimitiveComponent.CreateDynamicMaterialInstance` _skeletalmesh 0 "/Game/Weapon/Weapon_M/Com_Weapon_M.Com_Weapon_M" "None"))
  (`MaterialInstanceDynamic.SetTextureParameterValue` _returnvalue "Defuse" "/Game/Weapon/entry_s/horse/Horse_Brown_tem/Horse.Horse")
  (bind _returnvalue_2 (`PrimitiveComponent.CreateDynamicMaterialInstance` _skeletalmesh 1 "/Game/Weapon/Weapon_M/Com_Weapon_M.Com_Weapon_M" "None"))
  (`MaterialInstanceDynamic.SetTextureParameterValue` _returnvalue_2 "Defuse" "/Game/Weapon/entry_s/horse/Horse_Brown_tem/Horse_prom.Horse_prom"))

(fn `UserConstructionScript`
  (`parent.UserConstructionScript`))