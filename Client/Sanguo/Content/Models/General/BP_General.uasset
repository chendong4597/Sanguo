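; BP_General is a general unit with a widget HUD, a hero mount socket and input handling for clicking focus targets.
; On BeginPlay it hands itself to the HUD widget as owner.
; AttachHero finds the first BP_Hero in the level and snaps it to the mesh's S_Hero socket.
; Touch events feed GenHeroInputTouch, while left mouse press and release feed GenSightAround as Touch1 at the viewport cursor position.
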(event `self.ReceiveBeginPlay`
  (`parent.ReceiveBeginPlay`)
  (`self.InitHud`))

(event `self.AttachHero`
  ; hero attach
  (bind _outactors (`GameplayStatics.GetAllActorsOfClass` "/Game/Models/Player/BP_Hero.BP_Hero_C"))
  (if (> (`KismetArrayLibrary.Array_Length` _outactors) 0)
    (bind _output (`|GetArrayItem` _outactors))
    (`self.K2_DetachFromActor` _output "KeepRelative" "KeepWorld" "KeepRelative")
    (`self.K2_AttachToComponent` _output (`self.Mesh`) "S_Hero" "KeepRelative" "KeepWorld" "KeepRelative" true)
    (`self.K2_SetActorRelativeLocation` _output (0.0 0.0 0.0) false false)))

(event `InputTouch`
  (params (Location :type "Vector Structure") (FingerIndex :type "ETouchIndex Enum"))
  ;[1 1 1] 点击焦点目标
  (:`Pressed`
    (`self.GenHeroInputTouch` FingerIndex "Began" Location))
  (:`Released`
    (`self.GenHeroInputTouch` FingerIndex "Ended" Location))
  (:`Moved`
    (`self.GenHeroInputTouch` FingerIndex "Moved" Location)))

(event `Key|LeftMouseButton`
  (params (Key :type "Key Structure"))
  ;[1 1 1] 点击焦点目标
  (:`Pressed`
    (bind _returnvalue (`WidgetLayoutLibrary.GetMousePositionOnViewport`))
    (`self.GenSightAround` "Touch1" _returnvalue true))
  (:`Released`
    (bind _returnvalue_2 (`WidgetLayoutLibrary.GetMousePositionOnViewport`))
    (`self.GenSightAround` "Touch1" _returnvalue_2)))

(fn `InitHud`
  (bind _asbp_general_hud (cast `/Game/UI/BP_GeneralHud` (`WidgetComponent.GetWidget` (`self.GeneralHud`))))
  (`UIRoleHud.SetOwnerRole` _asbp_general_hud self))

(fn `UserConstructionScript`)