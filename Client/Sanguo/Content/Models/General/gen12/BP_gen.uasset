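; BP_gen is an actor Blueprint for the gen12 model that equips itself with a bone sword when play begins.
; After the parent BeginPlay, it spawns a BP_SwordBone actor and attaches it to the S_R_Hand socket on its Mesh, keeping relative transforms.
; The overlap and Tick events are disabled stubs, and the construction script only calls its parent.
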(event `self.ReceiveBeginPlay`
  (`parent.ReceiveBeginPlay`)
  (bind _returnvalue (`|SpawnActorFromClass` "/Game/Models/Weapon/entry_s/Sword/Sword_Bone/BP_SwordBone.BP_SwordBone_C" (`KismetMathLibrary.MakeTransform` (0.0 0.0 0.0)) "Undefined" "MultiplyWithRoot" null null))
  (`self.K2_AttachToComponent` _returnvalue (`self.Mesh`) "S_R_Hand" "KeepRelative" "KeepRelative" "KeepRelative" true))

(fn `UserConstructionScript`
  (`parent.UserConstructionScript`))