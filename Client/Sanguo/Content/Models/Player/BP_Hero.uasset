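; Player hero Blueprint that routes movement, touch and mouse input into hero functions defined outside this graph, such as PreWalk, Walk, HeroInputTouch and SightAround.
; Keyboard axes feed PreWalk, while BPWalk rotates a control-ball vector by spring arm yaw before calling Walk.
; Other events reset the spring arm's rotation, set its length as view distance, and pan the first CameraActor in the level along world X/Y.
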(event `self.ReceiveTick`
  (params (DeltaSeconds :type "Float (single-precision)")))

(event `InputAxis|MoveForward`
  (params (AxisValue :type "Float (single-precision)"))
  ;[1 1 1] PC键盘移动控制
  (`self.PreWalk` true AxisValue))

(event `InputAxis|MoveRight`
  (params (AxisValue :type "Float (single-precision)"))
  ;[1 1 1] PC键盘移动控制
  (`self.PreWalk` false AxisValue))

(event `self.BPWalk`
  (params (vec :type "Vector Structure"))
  (bind _returnvalue (`KismetMathLibrary.GetPI`))
  (bind (_returnvalue_roll _returnvalue_pitch _returnvalue_yaw) (`KismetMathLibrary.BreakRotator` (`SceneComponent.K2_GetComponentRotation` (`self.SpringArm`))))
  (bind _returnvalue_2 (+ (* 360 (/ (+ (/ (+ (`KismetMathLibrary.Atan2` vec_Y vec_X) _returnvalue) 2.0) (/ _returnvalue 2.0)) _returnvalue)) _returnvalue_yaw))
  ;[1 1 1] 控制球控制移动
  (`self.Walk` (`KismetMathLibrary.Normal` (`KismetMathLibrary.MakeVector` (`KismetMathLibrary.DegCos` _returnvalue_2) (`KismetMathLibrary.DegSin` _returnvalue_2)))))

(event `InputTouch`
  (params (Location :type "Vector Structure") (FingerIndex :type "ETouchIndex Enum"))
  ;[1 1 1] 点击焦点目标
  (:`Pressed`
    (`self.HeroInputTouch` FingerIndex "Began" Location))
  (:`Released`
    (`self.HeroInputTouch` FingerIndex "Ended" Location))
  (:`Moved`
    (`self.HeroInputTouch` FingerIndex "Moved" Location)))

(event `Key|LeftMouseButton`
  (params (Key :type "Key Structure"))
  ;[1 1 1] 点击焦点目标
  (:`Pressed`
    (bind _returnvalue (`WidgetLayoutLibrary.GetMousePositionOnViewport`))
    (`self.SightAround` "Touch1" _returnvalue true))
  (:`Released`
    (bind _returnvalue_2 (`WidgetLayoutLibrary.GetMousePositionOnViewport`))
    (`self.SightAround` "Touch1" _returnvalue_2)))

(event `self.Round`
  (params (bLeft :type Boolean) (fDelTm :type "Float (single-precision)"))
  ; Actor移动
  (bind _outactors (`GameplayStatics.GetAllActorsOfClass` "/Script/Engine.CameraActor"))
  (if (> (`KismetArrayLibrary.Array_Length` _outactors) 0)
    (if bLeft
      (bind _output (`|GetArrayItem` _outactors))
      (bind (_returnvalue_x _returnvalue_y _returnvalue_z) (`KismetMathLibrary.BreakVector` (`self.K2_GetActorLocation` _output)))
      (`self.K2_SetActorLocation` _output (`KismetMathLibrary.MakeVector` (+ _returnvalue_x fDelTm) _returnvalue_y _returnvalue_z) false false)
      (else
        (`self.K2_SetActorLocation` _output (`KismetMathLibrary.MakeVector` (- _returnvalue_x fDelTm) _returnvalue_y _returnvalue_z) false false)))))

(event `self.UpAndDown`
  (params (bUp :type Boolean) (fDelTm :type "Float (single-precision)"))
  ; Actor移动
  (bind _outactors (`GameplayStatics.GetAllActorsOfClass` "/Script/Engine.CameraActor"))
  (if (> (`KismetArrayLibrary.Array_Length` _outactors) 0)
    (if bUp
      (bind _output (`|GetArrayItem` _outactors))
      (bind (_returnvalue_x _returnvalue_y _returnvalue_z) (`KismetMathLibrary.BreakVector` (`self.K2_GetActorLocation` _output)))
      (`self.K2_SetActorLocation` _output (`KismetMathLibrary.MakeVector` _returnvalue_x (+ _returnvalue_y fDelTm) _returnvalue_z) false false)
      (else
        (`self.K2_SetActorLocation` _output (`KismetMathLibrary.MakeVector` _returnvalue_x (- _returnvalue_y fDelTm) _returnvalue_z) false false)))))

(event `self.EvtRecallHero`
  ; 重新设置回去
  (`SceneComponent.K2_SetWorldRotation` (`self.SpringArm`) (struct :`Pitch` -45.0 :`Yaw` 90.0) false false))

(event `self.Sight`
  (params (sightValue :type Integer))
  ; 设置视野
  (set `SpringArmComponent.TargetArmLength` (`KismetMathLibrary.Conv_IntToDouble` sightValue) (`self.SpringArm`)))

(fn `Move`
  (params (value :type "Float (double-precision)") (bLeft :type Boolean))
  ;[1 1 1] PC键盘移动控制
  (if (!= value 0.0)
    (if bLeft
      (`self.Walk` (`KismetMathLibrary.MakeVector` 0.0 1.0) value)
      (else
        (`self.Walk` (`KismetMathLibrary.MakeVector` -1.0) value)))))

(fn `UserConstructionScript`)